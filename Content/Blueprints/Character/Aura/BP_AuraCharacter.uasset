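; BP_AuraCharacter is the Aura character Blueprint, handling player camera zoom and rotation.
; The mouse wheel steps a clamped CameraPosition, which Tick converts into a spring arm length eased with FInterpTo, between the default and farther out.
; Holding the middle mouse button lets mouse movement add controller yaw and pitch, with horizontal movement also resetting control rotation roll to zero.
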(event `InputAxisKey|MouseWheelAxis`
  (params (AxisValue :type "Float (single-precision)"))
  (bind _maxcameraposition (`self.MaxCameraPosition`))
  ;[1 1 1] When mouse wheel scrolled
  (if (> AxisValue 0.0)
    (bind _result (`/Engine/EditorBlueprintResources/StandardMacros.IncrementInt` (`self.CameraPosition`))
      (:`  `
        (set `self.CameraPosition` (`KismetMathLibrary.Clamp` _result (* (`self.MaxCameraPosition`) -1)))))
    (elif (< AxisValue 0.0)
      (bind _result_2 (`/Engine/EditorBlueprintResources/StandardMacros.DecrementInt` (`self.CameraPosition`))
        (:`  `
          (set `self.CameraPosition` (`KismetMathLibrary.Clamp` _result_2 (* _maxcameraposition -1) _maxcameraposition)))))))

(event `self.ReceiveTick`
  (params (DeltaSeconds :type "Float (single-precision)"))
  (bind _springarm (`self.SpringArm`))
  ;[1 1 1] Set camera position while zooming/unzooming
  (set `SpringArmComponent.TargetArmLength` (`KismetMathLibrary.FInterpTo` (`SpringArmComponent.TargetArmLength` _springarm) (+ (`self.DefaultSpringArmLength`) (* (* (`self.CameraZoomDifference`) (`self.CameraPosition`)) -1.0)) DeltaSeconds 2.0) _springarm))

(event `Key|MiddleMouseButton`
  (params (Key :type "Key Structure"))
  ;[1 1 1] Turning camera
  (:`Pressed`
    (set `self.AllowCameraRotation` true))
  (:`Released`
    (set `self.AllowCameraRotation` false)))

(event `InputAxisKey|MouseX`
  (params (AxisValue :type "Float (single-precision)"))
  (bind (_returnvalue_roll _returnvalue_pitch _returnvalue_yaw) (`KismetMathLibrary.BreakRotator` (`self.GetControlRotation`)))
  ;[1 1 1] Turning camera
  (if (`self.AllowCameraRotation`)
    (`self.AddControllerYawInput` AxisValue)
    (`Controller.SetControlRotation` (`GameplayStatics.GetPlayerController` 0) (`KismetMathLibrary.MakeRotator` 0.0 _returnvalue_pitch _returnvalue_yaw))))

(event `InputAxisKey|MouseY`
  (params (AxisValue :type "Float (single-precision)"))
  ;[1 1 1] Turning camera
  (if (`self.AllowCameraRotation`)
    (bind _result (`/Engine/EditorBlueprintResources/StandardMacros.NegateFloat` AxisValue)
      (:`  `
        (`self.AddControllerPitchInput` _result)))))

(fn `UserConstructionScript`)